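; BP_ElecRobot is a level robot actor whose skeletal mesh animation is driven by externally triggered events.
; Wake-up plays the mesh's assigned animation once, while run, jump, mid-air, land and fly events each switch to a specific looping or one-shot animation, with no Anim Blueprint logic in the graph.
; GetRedBlueSpawner exposes the BP_RedBlueSpawner held in its child actor component.
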(event Custom|Trigger%20Wake%20Up
  (Audio|Components|Audio|Play (Variables|Default|GetSkeletalMesh) false))

(event Custom|Trigger%20Run
  (Components|Animation|PlayAnimation (Variables|Default|GetSkeletalMesh) "/Game/Cute_Robot/Animations/Anim_Sprint.Anim_Sprint" true))

(event Custom|Trigger%20Jump
  (Components|Animation|PlayAnimation (Variables|Default|GetSkeletalMesh) "/Game/Cute_Robot/Animations/Anim_Run_Jump.Anim_Run_Jump" false))

(event Custom|Trigger%20Mid%20Air
  (Components|Animation|PlayAnimation (Variables|Default|GetSkeletalMesh) "/Game/Cute_Robot/Animations/Anim_Jump_Middle.Anim_Jump_Middle" true))

(event Custom|Trigger%20Land
  (Components|Animation|PlayAnimation (Variables|Default|GetSkeletalMesh) "/Game/Cute_Robot/Animations/Anim_Jump_Land.Anim_Jump_Land" false))

(event Custom|Trigger%20Fly
  (Components|Animation|PlayAnimation (Variables|Default|GetSkeletalMesh) "/Game/Cute_Robot/Animations/Anim_Standing.Anim_Standing" true))

(event EventBeginPlay)

(event Collision|EventActorBeginOverlap
  (params (OtherActor :type Actor%20Object%20Reference)))

(event EventTick
  (params (DeltaSeconds :type Float%20%28single-precision%29)))

(fn ConstructionScript)

(fn GetRedBlueSpawner
  (bind _asbp_red_blue_spawner (Utilities|Casting|CastToBP_RedBlueSpawner (Variables|/Script/Engine.ChildActorComponent|GetChildActor (Variables|Default|GetRedBlueSpawner))))
  (return _asbp_red_blue_spawner))