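; BP_Sprite is a fire-level actor built to travel along a spline and drop colored balls, though that logic is currently disconnected.
; BeginPlay only stores the Cube's world location as the origin.
; Unwired graph fragments hold timeline-driven spline movement, spline-based rotation and an endless delayed loop alternating red and blue spawns.
; GenerateBall spawns BP_RedBall or BP_BlueBall below the actor, chosen by color.
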(event EventBeginPlay
  ;[1 1 1] Set Origin Location
  (Variables|Default|SetOriginLocation (Transformation|GetWorldLocation (Variables|Default|GetCube))))

(event Collision|EventActorBeginOverlap
  (params (OtherActor :type Actor%20Object%20Reference)))

(event EventTick
  (params (DeltaSeconds :type Float%20%28single-precision%29)))

(fn ConstructionScript)

(fn GenerateBall
  (params (BallColor :type ColorChoice%20Enum :default "NewEnumerator0"))
  (bind _returnvalue (Transformation|GetActorTransform))
  (bind _returnvalue_2 (+ (.location _returnvalue) "0,0,-150.000000"))
  (switch Utilities|FlowControl|Switch|SwitchonColorChoice BallColor
    (:NewEnumerator0
      (Game|SpawnActorfromClass "/Game/Levels/FireLevel/hudongyue/BP_RedBall.BP_RedBall_C" (Math|Transform|MakeTransform _returnvalue_2 (.rotation _returnvalue) (.scale _returnvalue)) "Undefined" 0 0))
    (:NewEnumerator1
      (Game|SpawnActorfromClass "/Game/Levels/FireLevel/hudongyue/BP_BlueBall.BP_BlueBall_C" (Math|Transform|MakeTransform _returnvalue_2 (.rotation _returnvalue) (.scale _returnvalue)) "Undefined" 0 0))))