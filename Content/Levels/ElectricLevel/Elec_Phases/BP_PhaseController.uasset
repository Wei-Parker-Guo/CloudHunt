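; BP_PhaseController runs a single phase of the electric level, with empty activate, deactivate and zero-returning accuracy functions that appear intended for child overrides.
; An ActorSequence drives the phase: triggering plays it, and resetting rewinds it to StartTime and restores state.
; The sequencer's Complete event, gated by IsComplete, ends the phase, reporting accuracy to ElectricLevelController.
; Restarting resets the phase and teleports the player to the location cached in Init.
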(event EventBeginPlay)

(event Collision|EventActorBeginOverlap
  (params (OtherActor :type Actor%20Object%20Reference)))

(event EventTick
  (params (DeltaSeconds :type Float%20%28single-precision%29)))

(event Custom|Complete
  (Development|PrintString (Utilities|String|ToString(Boolean) (Variables|Default|GetisComplete)))
  (if (Variables|Default|GetisComplete)
    (CallFunction|EndPhase)
    (Variables|Default|SetisComplete false)))

(fn ConstructionScript)

(fn Init
  (Variables|Default|SetStartLoc (Transformation|GetWorldLocation (Variables|Default|GetStartLocation))))

(fn ResetPhase
  (bind _actorsequence (Variables|Default|GetActorSequence))
  (bind _sequenceplayer (Variables|/Script/ActorSequence.ActorSequenceComponent|GetSequencePlayer _actorsequence))
  (Sequencer|Player|Stop _sequenceplayer :!class /Script/MovieScene.MovieSceneSequencePlayer)
  (Components|Timeline|SetPlaybackPosition _sequenceplayer (Utilities|Struct|MakeMovieSceneSequencePlaybackParams (Utilities|Struct|MakeFrameTime (Utilities|Struct|MakeFrameNumber 0) 0.0) (Variables|Default|GetStartTime) "" "Time" "Jump" false))
  (Class|MovieSceneSequencePlayer|RestoreState _sequenceplayer)
  (Variables|Default|SetReseted true)
  (Variables|Default|SetisComplete false))

(fn TriggerPhase
  (Sequencer|Player|Play (Variables|/Script/ActorSequence.ActorSequenceComponent|GetSequencePlayer (Variables|Default|GetActorSequence)) :!class /Script/MovieScene.MovieSceneSequencePlayer))

(fn EndPhase
  (bind _accuracy (CallFunction|GetAccuracy))
  (Default|CompletePhase (Variables|Default|GetElectricLevelController) _accuracy)
  (CallFunction|DeactivateController))

(fn DeactivateController)

(fn GetAccuracy
  (return 0.0))

(fn ActivateController)

(fn SpawnPlayeratStart
  (Transformation|SetActorLocation (Game|GetPlayerCharacter 0) (Variables|Default|GetStartLoc) false true))

(fn RestartPhase
  (CallFunction|ResetPhase)
  (CallFunction|SpawnPlayeratStart))