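; BP_CarSpawner spawns and manages a batch of cars on a track in the electric level.
; SpawnCar creates fifteen cars on CarTrack, staggering each start offset by index plus a scaled TimeDelay, and stores them in the Cars array.
; StartCar moves every stored car, while RemoveCar destroys them and resets the array.
; The event graph is unused, so these functions rely on external callers.
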(event EventBeginPlay)

(event Collision|EventActorBeginOverlap
  (params (OtherActor :type Actor%20Object%20Reference)))

(event EventTick
  (params (DeltaSeconds :type Float%20%28single-precision%29)))

(fn ConstructionScript)

(fn SpawnCar
  (params (timeDelay :type Float%20%28double-precision%29))
  (for _index (range 1 15)
    (bind _returnvalue (Game|SpawnActorfromClass "/Game/Levels/Elec_Ian/Elec3/Car.Car_C" (Math|Transform|MakeTransform "0, 0, 0" "0, 0, 0" "1.000000,1.000000,1.000000") "Undefined" 0 0))
    (Variables|/Game/Levels/Elec_Ian/Elec3/Car.Car_C|SetCarStartOffset _returnvalue (+ (* (Math|Conversions|ToFloat(Integer) _index) 0.041) (* timeDelay (/ 1.0 3e+02)) 0.015))
    (Variables|/Game/Levels/Elec_Ian/Elec3/Car.Car_C|SetCarTrack _returnvalue (Variables|Default|GetCarTrack))
    (Utilities|Array|Add (Variables|Default|GetCars) _returnvalue)))

(fn StartCar
  (for _array_element (Variables|Default|GetCars)
    (Default|MoveCar _array_element)))

(fn RemoveCar
  (for _array_element (Variables|Default|GetCars)
    (Actor|DestroyActor _array_element))
  (Variables|Default|SetCars (LocalVariables|GetEmpty%20Cars)))