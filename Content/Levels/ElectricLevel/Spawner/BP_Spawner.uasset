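; BP_Spawner tracks spawned balls, used as rhythm targets, and the player's accuracy on them in the Electric level.
; Each reported target leaves the BallSpawned set and adds to a running accuracy total and count, from which an average is returned.
; Helpers halve the total as a penalty, reset the score, or destroy all remaining balls.
; The event graph is empty, and no spawning logic appears here.
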(event EventBeginPlay)

(event Collision|EventActorBeginOverlap
  (params (OtherActor :type Actor%20Object%20Reference)))

(event EventTick
  (params (DeltaSeconds :type Float%20%28single-precision%29)))

(fn ConstructionScript)

(fn RemoveBall
  (params (toRemove :type BP%20Rythm%20Target%20Object%20Reference))
  (Utilities|Set|Remove (Variables|Default|GetBallSpawned) toRemove))

(fn RemoveAllBalls
  (bind _result (Utilities|Set|ToArray (Variables|Default|GetBallSpawned)))
  (for _array_element _result
    (if (Utilities|IsValid _array_element)
      (Actor|DestroyActor _array_element)))
  (Variables|Default|SetBallSpawned (LocalVariables|GetEmpty%20Set)))

(fn UpdateTotalAccuracy
  (params (Accuracy :type Float%20%28double-precision%29) (RythmTarget :type BP%20Rythm%20Target%20Object%20Reference))
  (CallFunction|RemoveBall RythmTarget)
  (Math|Integer|IncrementInt (Variables|Default|GetNumSpawned)
    (:%20%20
      (bind _output_get (Variables|Default|SetTotalAccuracy (+ (Variables|Default|GetTotalAccuracy) Accuracy))))))

(fn GetAverageAccuracy
  (return (/ (Variables|Default|GetTotalAccuracy) (Variables|Default|GetNumSpawned))))

(fn ApplyPenalty
  (Variables|Default|SetTotalAccuracy (/ (Variables|Default|GetTotalAccuracy) 2.0)))

(fn ResetAccuracy
  (Variables|Default|SetNumSpawned 0)
  (Variables|Default|SetTotalAccuracy 0.0))