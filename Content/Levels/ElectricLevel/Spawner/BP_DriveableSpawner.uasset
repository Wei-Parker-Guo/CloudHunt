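; Rhythm target spawner for the electric level, placing red/blue and purple targets along the driveable car's spline.
; On BeginPlay, Init precomputes a spline transform per beat time, using per-index lead times from the Long map or a default.
; Spawn functions consume these in beat order, set each target's normalized spline Alpha, randomly shift it into one of three lateral lanes, start it and track it in BallSpawned.
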(event EventBeginPlay
  (|CallParentFunction)
  (CallFunction|Init))

(event Collision|EventActorBeginOverlap
  (params (OtherActor :type Actor%20Object%20Reference))
  (|CallParentFunction OtherActor) ; This node is disabled and will not be called.\nDrag off pins to build functionality.
)

(fn ConstructionScript
  (|CallParentFunction))

(fn Init
  (for (_array_element _array_index) (Variables|Default|GetBeat%20Time)
    (if (.ReturnValue (Utilities|Map|Find (Variables|Default|Getlong) _array_index))
      (LocalVariables|Setdt (.Value (Utilities|Map|Find (Variables|Default|Getlong) _array_index)))
      (else
        (LocalVariables|Setdt 1.0)))
    (bind _transform (Default|LocationatSplineatTime (Variables|Default|GetDriveableCar) (- (+ _array_element (LocalVariables|Getdt)) (Variables|Default|GetStart%20Time))))
    (Utilities|Array|Add (Variables|Default|GetSpawn%20Transform) _transform)))

(fn SpawnRBTarget
  (params (TimeDelay :type Float%20%28double-precision%29))
  (bind _spawn_transform (Variables|Default|GetSpawn%20Transform))
  (bind _beat (Variables|Default|GetBeat))
  (bind _output (Utilities|Array|Get(acopy) _spawn_transform _beat))
  (Development|PrintString (Utilities|String|ToString(Transform) _output))
  (bind _returnvalue (Game|SpawnActorfromClass "/Game/Levels/BP_RedBlueDrivableTarget.BP_RedBlueDrivableTarget_C" _output "Undefined" 0 0))
  (Variables|/Game/Levels/BP_RedBlueDrivableTarget.BP_RedBlueDrivableTarget_C|SetAlpha _returnvalue (/ (- (+ (Utilities|Array|Get(acopy) (Variables|Default|GetBeat%20Time) _beat) 0.5) (Variables|Default|GetStart%20Time)) (Variables|/Game/Levels/ElectricLevel/DriveCar_Phase/BP_DriveableCar.BP_DriveableCar_C|GetDuration (Variables|Default|GetDriveableCar))))
  (Transformation|AddActorLocalOffset _returnvalue (Math|Vector|MakeVector 0.0 (Math|Conversions|ToFloat(Integer) (* (Math|Random|RandomIntegerinRange -1 1) 500)) 0.0) false false)
  (Variables|/Game/Levels/ElectricLevel/Elec_Rythm_Object/BP_RythmTarget.BP_RythmTarget_C|SetSpawner _returnvalue self)
  (Default|StartRedBlueTarget _returnvalue TimeDelay (Math|Random|RandomBool))
  (Utilities|Set|Add (Variables|Default|GetBallSpawned) _returnvalue)
  (Math|Integer|IncrementInt (Variables|Default|GetBeat)))

(fn GetAverageAccuracy
  (bind _average_accuray (|CallParentFunction))
  (return _average_accuray))

(fn SpawnPurpleTarget
  (params (TimeDelay :type Float%20%28double-precision%29))
  (bind _beat (Variables|Default|GetBeat))
  (bind _returnvalue (Game|SpawnActorfromClass "/Game/Levels/ElectricLevel/Elec_Rythm_Object/BP_PurpleRythmTarget.BP_PurpleRythmTarget_C" (Utilities|Array|Get(acopy) (Variables|Default|GetSpawn%20Transform) _beat) "Undefined" 0 0))
  (Variables|/Game/Levels/ElectricLevel/Elec_Rythm_Object/BP_PurpleRythmTarget.BP_PurpleRythmTarget_C|SetAlpha _returnvalue (/ (- (+ (Utilities|Array|Get(acopy) (Variables|Default|GetBeat%20Time) _beat) 2.0) (Variables|Default|GetStart%20Time)) (Variables|/Game/Levels/ElectricLevel/DriveCar_Phase/BP_DriveableCar.BP_DriveableCar_C|GetDuration (Variables|Default|GetDriveableCar))))
  (Transformation|AddActorLocalOffset _returnvalue (Math|Vector|MakeVector 0.0 (Math|Conversions|ToFloat(Integer) (* (Math|Random|RandomIntegerinRange -1 1) 500)) 0.0) false false)
  (Variables|/Game/Levels/ElectricLevel/Elec_Rythm_Object/BP_RythmTarget.BP_RythmTarget_C|SetSpawner _returnvalue self)
  (Default|StartPurpleTarget _returnvalue 1.0 TimeDelay)
  (Utilities|Set|Add (Variables|Default|GetBallSpawned) _returnvalue)
  (Math|Integer|IncrementInt (Variables|Default|GetBeat)))