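; BP_BomController is a phase controller for the BomBom phase of the Electric Level, driving bomb spawns against a crashable building.
; Sequencer events tell the Spawner to spawn bombs from per-beat time and height arrays, crash the Building, and complete the phase.
; Player overlaps with trigger volumes reset the level state or flag completion.
; Resetting clears balls, re-enables triggers and respawns the Building if destroyed, while accuracy comes from the Spawner's average.
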(event OnComponentBeginOverlap(OutOfBound)
  (params (OverlappedComponent :type Primitive%20Component%20Object%20Reference) (OtherActor :type Actor%20Object%20Reference) (OtherComp :type Primitive%20Component%20Object%20Reference) (OtherBodyIndex :type Integer) (bFromSweep :type Boolean) (SweepResult :type Hit%20Result%20Structure%20%28by%20ref%29))
  (Development|PrintString "Hello")
  (if (== (Utilities|GetClass OtherActor) "/Game/AdvancedLocomotionV4/Blueprints/CharacterLogic/ALS_Player.ALS_Player_C")
    (Utilities|FlowControl|DoOnce false :!label _label
      (:Completed
        (CallFunction|OverlapOutOfBound)
        (Development|PrintString "RESEETTTTTT")
        (goto _label Reset)))))

(event OnComponentBeginOverlap(End)
  (params (OverlappedComponent :type Primitive%20Component%20Object%20Reference) (OtherActor :type Actor%20Object%20Reference) (OtherComp :type Primitive%20Component%20Object%20Reference) (OtherBodyIndex :type Integer) (bFromSweep :type Boolean) (SweepResult :type Hit%20Result%20Structure%20%28by%20ref%29))
  (Development|PrintString "Hello")
  (if (== (Utilities|GetClass OtherActor) "/Game/AdvancedLocomotionV4/Blueprints/CharacterLogic/ALS_Player.ALS_Player_C")
    (Utilities|FlowControl|DoOnce false :!label _label
      (:Completed
        (Variables|Default|SetisComplete true)
        (goto _label Reset)))))

(event EventBeginPlay
  (CallFunction|Init))

(event EventTick
  (params (DeltaSeconds :type Float%20%28single-precision%29)))

(event Custom|Spawn
  (bind _beatcounter (Variables|Default|GetBeatCounter))
  (Default|SpawnBom (Variables|Default|GetSpawner) (Utilities|Array|Get(acopy) (Variables|Default|GetBeatTime) _beatcounter) (Utilities|Array|Get(acopy) (Variables|Default|GetHeigtRate) _beatcounter))
  (Math|Integer|IncrementInt _beatcounter))

(event Custom|BaoZha
  (Collision|SetCollisionEnabled (Variables|Default|GetOutOfBound) "NoCollision")
  (Default|Crash (Variables|Default|GetBuilding)))

(event Custom|Complete%20Bom
  (CallFunction|Complete))

(fn ConstructionScript)

(fn Init
  (Variables|/Game/Levels/ElectricLevel/Spawner/BP_Spawner.BP_Spawner_C|SetPhaseController (Variables|Default|GetSpawner) self)
  (Variables|Default|SetBuilding%20Transform (Transformation|GetActorTransform (Variables|Default|GetBuilding)))
  (|CallParentFunction))

(fn ResetPhase
  (Variables|Default|SetBeatCounter 0)
  (CallFunction|SpawnBuilding)
  (CallFunction|EnableCollision)
  (Default|RemoveAllBalls (Variables|Default|GetSpawner))
  (|CallParentFunction))

(fn OverlapOutOfBound
  (Default|ResetCurrentState (Variables|Default|GetElectricLevelController)))

(fn TriggerPhase
  (|CallParentFunction))

(fn EndPhase
  (|CallParentFunction)
  (Default|ResetAccuracy (Variables|Default|GetSpawner))
  (CallFunction|SpawnBuilding))

(fn GetAccuracy
  (bind _average_accuray (Default|GetAverageAccuracy (Variables|Default|GetSpawner)))
  (return _average_accuray))

(fn DeactivateController
  (CallFunction|DisableCollision)
  (|CallParentFunction))

(fn ActivateController
  (CallFunction|ResetPhase)
  (|CallParentFunction))

(fn SpawnBuilding
  (if (not (Utilities|IsValid (Variables|Default|GetBuilding)))
    (bind _returnvalue (Game|SpawnActorfromClass "/Game/Levels/ElectricLevel/Building.Building_C" (Variables|Default|GetBuilding%20Transform) "Undefined" 0 0))
    (Variables|Default|SetBuilding _returnvalue)))

(fn EnableCollision
  (Collision|SetCollisionEnabled (Variables|Default|GetEnd) "QueryOnly")
  (Collision|SetCollisionEnabled (Variables|Default|GetOutOfBound) "QueryOnly"))

(fn DisableCollision
  (Collision|SetCollisionEnabled (Variables|Default|GetEnd) "NoCollision")
  (Collision|SetCollisionEnabled (Variables|Default|GetOutOfBound) "NoCollision"))