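; Shootable rhythm target in the electric level that scores how close a hit lands to its beat time.
; StartTarget plays a color and scale timeline paced to twice the delay, signaling the timing window.
; A one-time Hit computes normalized accuracy, plays explosion and drum sound, hides the target, spawns feedback text and reports to the Spawner.
; If unshot when the timeline finishes, it reports a miss, then destroys itself either way.
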(event Custom|Start%20Target
  (params (Time%20Delay :type Float%20%28double-precision%29))
  (Variables|Default|SetStartTime (Actor|GetGameTimeSinceCreation))
  (CallFunction|StartBillboard (Variables|Default|GetTarget%20Reference))
  (Variables|Default|SetTimeDelay Time%20Delay)
  (Components|Timeline|SetPlayRate (Variables|Default|GetRythm%20Indication) (/ 1.0 (* Time%20Delay 2.0)))
  (bind (_direction _color_change _targetsize) (Timeline|Rythm%20Indication Play)
    (:Update
      (Rendering|Material|SetVectorParameterValueonMaterials (Variables|Default|GetRythm%20Target) "Color" (Math|Vector|MakeVector (.r _color_change) (.g _color_change) (.b _color_change)))
      (Transformation|SetRelativeScale3D (Variables|Default|GetTarget) (Math|Vector|MakeVector _targetsize _targetsize 1.0)))
    (:Finished
      (if (Variables|Default|GetisShot)
        _
        (else
          (CallFunction|MissTarget)))
      (Actor|DestroyActor))
    (:DestroyTarget
      (Development|SetHiddeninGame (Variables|Default|GetTarget) true false))))

(event EventBeginPlay)

(event EventHit
  (params (isBlueBullet :type Boolean))
  (Utilities|FlowControl|DoOnce false
    (:Completed
      (Collision|SetActorEnableCollision false)
      (CallFunction|Update))))

(fn ConstructionScript)

(fn CalculateAccuracy
  (bind _timedelay (Variables|Default|GetTimeDelay))
  ;[1 1 1] Accuracy = elapsed time
  (return (- 1.0 (/ (Math|Float|Absolute(Float) (- (- (Actor|GetGameTimeSinceCreation) (Variables|Default|GetStartTime)) _timedelay)) _timedelay))))

(fn Update
  (bind _returnvalue (Transformation|GetActorLocation))
  (bind _accuracy (CallFunction|CalculateAccuracy))
  (LocalVariables|SetAccuracy _accuracy)
  (Effects|SpawnEmitteratLocation "/Game/StarterContent/Particles/P_Explosion.P_Explosion" _returnvalue "0, 0, 0" "2.000000,2.000000,2.000000")
  (Audio|SpawnSoundatLocation "/Game/Levels/ElectricLevel/drum_stick_hit_sound.drum_stick_hit_sound" _returnvalue "0, 0, 0" 1.0 1.0 0.0 0 0)
  (CallFunction|SpawnFeedback (LocalVariables|GetAccuracy))
  (Rendering|SetActorHiddenInGame true)
  (Collision|SetCollisionEnabled (Variables|Default|GetSphere) "NoCollision")
  (CallFunction|UpdateSpawner (LocalVariables|GetAccuracy))
  (Variables|Default|SetisShot true))

(fn MissTarget
  (CallFunction|SpawnFeedback -1.0)
  (CallFunction|UpdateSpawner 0.0))

(fn UpdateSpawner
  (params (Accuracy :type Float%20%28double-precision%29))
  (Default|UpdateTotalAccuracy (Variables|Default|GetSpawner) Accuracy self))

(fn SpawnFeedback
  (params (Accuracy :type Float%20%28double-precision%29))
  (bind _returnvalue (Game|SpawnActorfromClass "/Game/Levels/ElectricLevel/Elec_Rythm_Object/BP_RythmAccFB.BP_RythmAccFB_C" (Math|Transform|MakeTransform (Transformation|GetActorLocation) "0, 0, 0" "1.000000,1.000000,1.000000") "Undefined" 0 0))
  (Default|UpdateText _returnvalue Accuracy))